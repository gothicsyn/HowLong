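; BPC_Health is a Blueprint component that tracks a current health value.
; RemoveHealth and Addhealth subtract or add a given amount, clamping the result between the minimum and maximum health.
; The event graph has no active logic, and neither function broadcasts changes or handles death.
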(fn `Addhealth`
  (params (Amount :type "Float (double-precision)"))
  (set `self.currentHealth` (`KismetMathLibrary.FClamp` (+ Amount (`self.currentHealth`)) (`self.minHealth`) (`self.maxHealth`))))

(fn `RemoveHealth`
  (params (Amount :type "Float (double-precision)"))
  (set `self.currentHealth` (`KismetMathLibrary.FClamp` (- (`self.currentHealth`) Amount) (`self.minHealth`) (`self.maxHealth`))))