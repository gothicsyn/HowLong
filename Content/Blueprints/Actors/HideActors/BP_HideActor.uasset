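; Interactable hiding spot actor that moves the player between its HidingPosition and ExitPosition, toggled by the player's IsHiding state.
; Entering disables player collision, movement and inventory access, and completing an exit restores them.
; Interact starts a looping frame-delta timer that slides the player at constant speed with VInterpToConstant.
; On arrival it clears the timers, fires the FinishedMoving dispatcher and flips IsHiding.
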(event `self.ReceiveBeginPlay`
  (bind _asl1_character (cast `/Game/GameBP/Level1/L1_Character` (`GameplayStatics.GetPlayerCharacter` 0)))
  (set `self.PlayerRef` _asl1_character)
  (bind _ashg_player_controller (cast `/Game/GameBP/HG_PlayerController` (`GameplayStatics.GetPlayerController` 0)))
  (set `self.controllerRef` _ashg_player_controller))

(event `/Game/Blueprints/Interfaces/BPI_Interaction.Interact`
  (bind _playerref (`self.PlayerRef`))
  (if (`/Game/GameBP/Level1/L1_Character.isHiding` (`self.PlayerRef`))
    (bind _returnvalue (`KismetSystemLibrary.K2_SetTimerDelegate` (delegate `MoveCharacter`) (`GameplayStatics.GetWorldDeltaSeconds`) true))
    (else
      (`self.SetActorEnableCollision` _playerref false)
      (`CharacterMovementComponent.DisableMovement` (`Character.CharacterMovement` _playerref))
      (set `/Game/GameBP/HG_PlayerController.canOpenInventory` false (`self.controllerRef`))
      (bind _returnvalue_2 (`KismetSystemLibrary.K2_SetTimerDelegate` (delegate `MoveCharacter`) (`GameplayStatics.GetWorldDeltaSeconds`) true)))))

(event `MoveCharacter`
  (bind _playerref (`self.PlayerRef`))
  (`self.K2_SetActorTransform` _playerref (`KismetMathLibrary.MakeTransform` (`KismetMathLibrary.VInterpTo_Constant` (`self.K2_GetActorLocation` _playerref) (`SceneComponent.K2_GetComponentLocation` (select `bool` (`/Game/GameBP/Level1/L1_Character.isHiding` (`self.PlayerRef`)) :`false` (`self.HidingPosition`) :`true` (`self.ExitPosition`) :!type "SceneComponent Object Reference")) (`GameplayStatics.GetWorldDeltaSeconds`) 1000.0)) false false)
  (if (== (`self.K2_GetActorLocation` (`self.PlayerRef`)) (`SceneComponent.K2_GetComponentLocation` (select `bool` (`/Game/GameBP/Level1/L1_Character.isHiding` (`self.PlayerRef`)) :`false` (`self.HidingPosition`) :`true` (`self.ExitPosition`) :!type "SceneComponent Object Reference")) :`ErrorTolerance` 0.01)
    (`KismetSystemLibrary.K2_ClearAndInvalidateTimerHandle` (stale `/Game/Blueprints/Interfaces/BPI_Interaction.Interact` _returnvalue_2))
    (`KismetSystemLibrary.K2_ClearAndInvalidateTimerHandle` (stale `/Game/Blueprints/Interfaces/BPI_Interaction.Interact` _returnvalue))
    (`self.FinishedMoving`)))

(event `FinishedMoving`
  (bind _playerref (`self.PlayerRef`))
  (bind _playerref_2 (`self.PlayerRef`))
  (`self.FinishedMovingED`)
  (if (`/Game/GameBP/Level1/L1_Character.isHiding` _playerref)
    (set `/Game/GameBP/Level1/L1_Character.isHiding` false _playerref)
    (`self.SetActorEnableCollision` _playerref_2 true)
    (`CharacterMovementComponent.SetMovementMode` (`Character.CharacterMovement` _playerref_2) "MOVE_Walking" 0)
    (set `/Game/GameBP/HG_PlayerController.canOpenInventory` true (`self.controllerRef`))
    (else
      (set `/Game/GameBP/Level1/L1_Character.isHiding` true _playerref))))

(fn `UserConstructionScript`)